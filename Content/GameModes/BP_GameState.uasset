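; Game state for a two-sided, turn-based number guessing game, alternating between server and client.
; Three seconds after BeginPlay, it sets chat window buttons according to Turn and network authority; NextTurn flips Turn, whose OnRep is empty.
; It passes the generated answer to the local player controller and routes guesses and ball counts through the chat widget into the controller's Enter.
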(event Custom|SetGeneratedNumber
  (params (GeneratedNumber :type Array%20of%20Integers))
  (bind _output_get (Variables|Default|SetGSRandomNums GeneratedNumber))
  (bind _asbp_controller (Utilities|Casting|CastToBP_Controller (Game|GetPlayerController 0)))
  (Default|SetAnswer _asbp_controller _output_get))

(event Custom|EnterClicked
  (bind _foundwidgets (Widget|GetAllWidgetsOfClass "/Game/Widgets/WBP_ChatWindow.WBP_ChatWindow_C" true))
  (bind _output_get (Variables|/Game/Widgets/WBP_ChatWindow.WBP_ChatWindow_C|SetGuessNumber (Utilities|Array|Get(acopy) _foundwidgets) (Variables|Default|GetGuessNum)))
  (bind _output_get_2 (Variables|/Game/Widgets/WBP_ChatWindow.WBP_ChatWindow_C|SetSTBall (Utilities|Array|Get(acopy) _foundwidgets) (Variables|Default|GetBallcount)))
  (bind _asbp_controller (Utilities|Casting|CastToBP_Controller (Game|GetPlayerController 0)))
  (Default|Enter _asbp_controller _output_get _output_get_2))

(event Custom|NextTurn
  (if (== (Variables|Default|GetTurn) 0)
    (Variables|Default|SetTurn 1)
    (Development|PrintString "클라턴")
    (else
      (Variables|Default|SetTurn 0)
      (Development|PrintString "서버턴"))))

(event Custom|TurnChanged)

(event Custom|TurnOffButton
  (Utilities|Casting|CastToBP_GameState (Game|GetGameState))
  (bind _foundwidgets (Widget|GetAllWidgetsOfClass "/Game/Widgets/WBP_ChatWindow.WBP_ChatWindow_C" true))
  (Default|TurnOffButton _foundwidgets))

(event Custom|TurnOnButton
  (Utilities|Casting|CastToBP_GameState (Game|GetGameState))
  (bind _foundwidgets (Widget|GetAllWidgetsOfClass "/Game/Widgets/WBP_ChatWindow.WBP_ChatWindow_C" true))
  (Default|TurnonButton _foundwidgets))

(event EventBeginPlay
  (Utilities|FlowControl|Delay 3.0)
  (if (== (Variables|Default|GetTurn) 0)
    (Utilities|Casting|CastToBP_GameState (Game|GetGameState))
    (Utilities|Casting|CastToBP_Controller (Game|GetPlayerController 0))
    (Networking|SwitchHasAuthority
      (:Remote
        (bind _foundwidgets (Widget|GetAllWidgetsOfClass "/Game/Widgets/WBP_ChatWindow.WBP_ChatWindow_C" true))
        (Default|TurnOffButton _foundwidgets)))
    (else
      (Utilities|Casting|CastToBP_GameState (Game|GetGameState))
      (bind _foundwidgets_2 (Widget|GetAllWidgetsOfClass "/Game/Widgets/WBP_ChatWindow.WBP_ChatWindow_C" true))
      (Default|TurnOffButton _foundwidgets_2)
      (Utilities|Casting|CastToBP_Controller (Game|GetPlayerController 0))
      (Networking|SwitchHasAuthority
        (:Remote
          (bind _foundwidgets_3 (Widget|GetAllWidgetsOfClass "/Game/Widgets/WBP_ChatWindow.WBP_ChatWindow_C" true))
          (Default|TurnonButton _foundwidgets_3))))))

(fn ConstructionScript)

(fn OnRepTurn)