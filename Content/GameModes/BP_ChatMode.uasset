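; BP_ChatMode is a game mode that sets up the opening turn and random numbers for a server/client match.
; On BeginPlay it randomly writes server or client turn to BP_GameState and prints which.
; After a short delay it calls GenerateRandomNumbers, stores the result and passes it to the game state through SetGeneratedNumber.
; A custom event quits the game; Tick and OnRep_RandomNums are empty.
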(event Custom|커스텀이벤트
  (Game|QuitGame 0 "Quit" false))

(event EventBeginPlay
  (bind _asbp_game_state (Utilities|Casting|CastToBP_GameState (Game|GetGameState)))
  (bind _output_get (Variables|/Game/GameModes/BP_GameState.BP_GameState_C|SetTurn _asbp_game_state (Math|Random|RandomIntegerinRange 0 1)))
  (if (== _output_get 0)
    (Development|PrintString "서버턴")
    (else
      (Development|PrintString "클라턴")))
  (Utilities|FlowControl|Delay 3.0)
  (bind _returnvalue (Class|CTBlueprintFunctionLibrary|GenerateRandomNumbers))
  (bind _output_get_2 (Variables|Default|SetGMRandomNums _returnvalue))
  (bind _asbp_game_state_2 (Utilities|Casting|CastToBP_GameState (Game|GetGameState)))
  (Default|SetGeneratedNumber _asbp_game_state_2 _output_get_2))

(event EventTick
  (params (DeltaSeconds :type Float%20%28single-precision%29)))

(fn ConstructionScript)

(fn OnRepRandomNums)