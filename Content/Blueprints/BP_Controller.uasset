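; Player controller for a turn-based multiplayer number-guessing game with ball counts, played through a chat-window widget.
; On BeginPlay it enables UI-only input and creates WBP_ChatWindow for the local player.
; Events push answers and guess results into that widget, and forward guesses, ball counts and turn requests to BP_GameState.
; Button toggling and IsMyTurn use network authority to tell the two sides apart, with turn 0 as a special case.
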(event Custom|Enter
  (params (GuessNum :type Text) (BallCount :type Text))
  (bind _foundwidgets (Widget|GetAllWidgetsOfClass "/Game/Widgets/WBP_ChatWindow.WBP_ChatWindow_C" true))
  (Variables|/Game/Widgets/WBP_ChatWindow.WBP_ChatWindow_C|SetGuessNumber (Utilities|Array|Get(acopy) _foundwidgets) GuessNum)
  (Variables|/Game/Widgets/WBP_ChatWindow.WBP_ChatWindow_C|SetSTBall (Utilities|Array|Get(acopy) _foundwidgets) BallCount)
  (Default|UIEnter (Utilities|Array|Get(acopy) _foundwidgets)))

(event Custom|SetAnswer
  (params (RandomNums :type Array%20of%20Integers))
  (Utilities|FlowControl|Delay 0.2)
  (bind _foundwidgets (Widget|GetAllWidgetsOfClass "/Game/Widgets/WBP_ChatWindow.WBP_ChatWindow_C" true))
  (Variables|/Game/Widgets/WBP_ChatWindow.WBP_ChatWindow_C|SetAnswer (Utilities|Array|Get(acopy) _foundwidgets) RandomNums)
  (Default|ShowAnswer (Utilities|Array|Get(acopy) _foundwidgets)))

(event Custom|ServerGetGameState
  (bind _asbp_game_state (Utilities|Casting|CastToBP_GameState (Game|GetGameState)))
  (Default|EnterClicked _asbp_game_state))

(event Custom|CustomEvent
  (Utilities|Casting|CastToBP_GameState (Game|GetGameState))
  (Networking|SwitchHasAuthority
    (:Authority
      (bind _foundwidgets (Widget|GetAllWidgetsOfClass "/Game/Widgets/WBP_ChatWindow.WBP_ChatWindow_C" true))
      (Default|TurnonButton _foundwidgets))))

(event Custom|UpdateGuessNum
  (params (GuessNum :type Text))
  (bind _asbp_game_state (Utilities|Casting|CastToBP_GameState (Game|GetGameState)))
  (Variables|/Game/GameModes/BP_GameState.BP_GameState_C|SetGuessNum _asbp_game_state GuessNum))

(event Custom|CustomEvent_1
  (bind _asbp_game_state (Utilities|Casting|CastToBP_GameState (Game|GetGameState)))
  (Default|TurnonButton _asbp_game_state))

(event Custom|UpdateBallCount
  (params (BallCount :type Text))
  (bind _asbp_game_state (Utilities|Casting|CastToBP_GameState (Game|GetGameState)))
  (Variables|/Game/GameModes/BP_GameState.BP_GameState_C|SetBallcount _asbp_game_state BallCount))

(event Custom|RequestNextTurn
  (bind _asbp_game_state (Utilities|Casting|CastToBP_GameState (Game|GetGameState)))
  (Default|NextTurn _asbp_game_state))

(event Custom|커스텀이벤트
  (bind _asbp_chat_mode (Utilities|Casting|CastToBP_ChatMode (Game|GetGameMode)))
  (Default|커스텀이벤트 _asbp_chat_mode))

(event Custom|OnOffButton
  (bind _asbp_game_state (Utilities|Casting|CastToBP_GameState (Game|GetGameState)))
  (if (== (Variables|/Game/GameModes/BP_GameState.BP_GameState_C|GetTurn _asbp_game_state) 0)
    (CallFunction|CustomEvent1)
    (Networking|SwitchHasAuthority
      (:Authority
        (bind _foundwidgets (Widget|GetAllWidgetsOfClass "/Game/Widgets/WBP_ChatWindow.WBP_ChatWindow_C" true))
        (Default|TurnOffButton _foundwidgets)))
    (else
      (Networking|SwitchHasAuthority
        (:Remote
          (bind _foundwidgets_2 (Widget|GetAllWidgetsOfClass "/Game/Widgets/WBP_ChatWindow.WBP_ChatWindow_C" true))
          (Default|TurnOffButton _foundwidgets_2)
          (CallFunction|CustomEvent))))))

(event EventBeginPlay
  (Variables|Default|SetbShowMouseCursor true)
  (Input|SetInputModeUIOnly (Game|GetPlayerController 0) 0 "DoNotLock" false)
  (if (Pawn|IsLocalController)
    (bind _returnvalue (UserInterface|CreateWidget "/Game/Widgets/WBP_ChatWindow.WBP_ChatWindow_C"))
    (UserInterface|Viewport|AddtoViewport _returnvalue 0)))

(fn ConstructionScript)

(fn IsMyTurn
  (if (Ability|HasAuthority)
    (Utilities|Casting|CastToBP_GameState (Game|GetGameState))
    (return 0)
    (else
      (Utilities|Casting|CastToBP_GameState (Game|GetGameState))
      (return 1))))